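; BP_Pickup is a points pickup that pulls itself toward the player and awards its delegated points when collected.
; Overlapping the SuckCollider with a BP_PlayerBase stores that player, and Tick then lerps the pickup toward them at SuckSpeed.
; PickupInterface shows the value on its WBP_TextPoints widget, hides the sprite and adds the points to the player and HUD.
; A short timer then calls DestroySelf.
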(event OnComponentBeginOverlap(SuckCollider)
  (params (OverlappedComponent :type Primitive%20Component%20Object%20Reference) (OtherActor :type Actor%20Object%20Reference) (OtherComp :type Primitive%20Component%20Object%20Reference) (OtherBodyIndex :type Integer) (bFromSweep :type Boolean) (SweepResult :type Hit%20Result%20Structure%20%28by%20ref%29))
  ;[1 1 1] Suck collider
  (bind _asbp_player_base (Utilities|Casting|CastToBP_PlayerBase OtherActor))
  (Variables|Default|SetPlayerRef _asbp_player_base)
  (Variables|Default|SetInRange true))

(event EventTick
  (params (DeltaSeconds :type Float%20%28single-precision%29))
  (bind _playerref (Variables|Default|GetPlayerRef))
  ;[1 1 1] Suck collider
  (if (Variables|Default|GetInRange)
    (Utilities|IsValid _playerref
      (:Is%20Valid
        (Transformation|SetActorLocation (Math|Vector|Lerp(Vector) (Transformation|GetActorLocation) (Transformation|GetActorLocation _playerref) (* (Variables|Default|GetSuckSpeed) DeltaSeconds)) false false)))))

(event EventMakeWidget
  (if (Utilities|DoesObjectImplementInterface (Variables|Default|GetOverlappedActor) "/Game/Blueprints/BP_PickupInterface.BP_PickupInterface_C")
    (CallFunction|PickupInterface)))

(fn ConstructionScript)

(fn DestroySelf
  (Actor|DestroyActor))

(fn PickupInterface
  (bind _aswbp_text_points (Utilities|Casting|CastToWBP_TextPoints (UserInterface|GetUserWidgetObject (Variables|Default|GetPointText))))
  (Utilities|IsValid _aswbp_text_points
    (:Is%20Valid
      (Default|UpdatePointsDisplayed _aswbp_text_points (Utilities|Text|ToText(String) (Utilities|String|Append "+" (Utilities|String|ToString(Integer) (Variables|Default|GetPointsDelegated)))))
      (Rendering|SetVisibility (Variables|Default|GetSprite) false false)
      (bind _asbp_player_base (Utilities|Casting|CastToBP_PlayerBase (Game|Player|GetPlayerPawn 0)))
      (Utilities|IsValid _asbp_player_base
        (:Is%20Valid
          (bind _output_get (Variables|/Script/Platformer.PlayerPaperCharacter|SetPoints _asbp_player_base (+ (Variables|/Script/Platformer.PlayerPaperCharacter|GetPoints _asbp_player_base) (Variables|Default|GetPointsDelegated))))
          (Default|UpdatePoints (Variables|/Game/Blueprints/Player/BP_PlayerBase.BP_PlayerBase_C|GetHUDRef _asbp_player_base) _output_get)
          (Utilities|Time|SetTimerbyFunctionName 0 "DestroySelf" 2.0)
          (return true))))))