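; Game mode for a platformer that handles level progression and carries the player's score between levels.
; On BeginPlay in any level except Level1, it restores the level index and the player's points from a LevelSave slot.
; TryLoadNextLevel increments the index, saves it with the score, and opens the next map by building its name from "Level" plus the number.
; At the final level it runs RestartLevel instead.
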(event Custom|TryLoadNextLevel
  (params (PlayerRef :type BP%20Player%20Base%20Object%20Reference))
  (Variables|Default|SetPlayer%20Ref PlayerRef)
  (if (< (Variables|Default|GetCurrentLevel) (Variables|Default|GetTotalLevels))
    (bind _result (Math|Integer|IncrementInt (Variables|Default|GetCurrentLevel))
      (:%20%20
        (Variables|Default|SetCurrentLevel _result)
        (bind _returnvalue (SaveGame|CreateSaveGameObject "/Game/Assets/LevelSave.LevelSave_C"))
        (bind _output_get (Variables|Default|SetLevelSave _returnvalue))
        (Utilities|IsValid (Variables|Default|GetPlayer%20Ref)
          (:Is%20Valid
            (Variables|/Game/Assets/LevelSave.LevelSave_C|SetScore _output_get (Variables|/Script/Platformer.PlayerPaperCharacter|GetPoints (Variables|Default|GetPlayer%20Ref)))
            (Variables|/Game/Assets/LevelSave.LevelSave_C|SetCurrentLevel _output_get (Variables|Default|GetCurrentLevel))
            (SaveGame|SaveGametoSlot _output_get (Variables|Default|GetSlot%20Name))
            (Game|OpenLevel(byName) (Utilities|String|StringToName (Utilities|String|Append "Level" (Utilities|String|ToString(Integer) (Variables|Default|GetCurrentLevel)))))))))
    (else
      (Development|ExecuteConsoleCommand "RestartLevel" 0))))

(event EventBeginPlay
  (bind _returnvalue (Game|GetCurrentLevelName true))
  (if (not (Utilities|Enum|Equal(Enum) _returnvalue "Level1"))
    (bind _returnvalue_2 (Actor|GetActorOfClass "/Game/Blueprints/Player/BP_PlayerBase.BP_PlayerBase_C"))
    (Variables|Default|SetPlayer%20Ref _returnvalue_2)
    (bind _returnvalue_3 (SaveGame|LoadGamefromSlot (Variables|Default|GetSlot%20Name)))
    (bind _aslevel_save (Utilities|Casting|CastToLevelSave _returnvalue_3))
    (Variables|Default|SetCurrentLevel (Variables|/Game/Assets/LevelSave.LevelSave_C|GetCurrentLevel _aslevel_save))
    (Variables|/Script/Platformer.PlayerPaperCharacter|SetPoints (Variables|Default|GetPlayer%20Ref) (Variables|/Game/Assets/LevelSave.LevelSave_C|GetScore _aslevel_save))))

(fn ConstructionScript)