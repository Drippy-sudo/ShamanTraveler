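; BP_EnemyBat is a side-scrolling bat enemy that starts in a random horizontal direction and moves continuously along X.
; Non-player hits with a horizontal normal reverse it and mirror the sprite, debounced by a delayed DoOnce reset.
; Projectile overlaps briefly halt it and show a Stunned indicator.
; Its EnemyDied override displays and awards points, updates the HUD, spawns smoke, hides the bat and destroys it after a timer.
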(event OnComponentHit(CapsuleComponent)
  (params (HitComponent :type Primitive%20Component%20Object%20Reference) (OtherActor :type Actor%20Object%20Reference) (OtherComp :type Primitive%20Component%20Object%20Reference) (NormalImpulse :type Vector :default "0, 0, 0") (Hit :type Hit%20Result%20Structure%20%28by%20ref%29))
  (if (!= OtherActor (Game|Player|GetPlayerPawn 0))
    (if (!= (.X (Math|Vector|BreakVector (.normal Hit))) 0.0)
      (Utilities|FlowControl|DoOnce false
        (:Completed
          (Variables|Default|SetbMoveRight (not (Variables|Default|GetbMoveRight)))
          (CallFunction|ToggleFacingDirection)
          (Utilities|FlowControl|Delay 0.2)
          (CallFunction|ResetDirectionChangeCheck))))))

(event OnComponentBeginOverlap(CapsuleComponent)
  (params (OverlappedComponent :type Primitive%20Component%20Object%20Reference) (OtherActor :type Actor%20Object%20Reference) (OtherComp :type Primitive%20Component%20Object%20Reference) (OtherBodyIndex :type Integer) (bFromSweep :type Boolean) (SweepResult :type Hit%20Result%20Structure%20%28by%20ref%29))
  (Utilities|Casting|CastToBP_Projectile OtherActor)
  (Rendering|SetVisibility (Variables|Default|GetStunned) true false)
  (Variables|Default|SetbCanMove false)
  (Variables|/Script/Engine.MovementComponent|SetVelocity (Variables|Character|GetCharacterMovement) "0, 0, 0")
  (Utilities|FlowControl|Delay 1.0)
  (Variables|Default|SetbCanMove true)
  (Rendering|SetVisibility (Variables|Default|GetStunned) false false))

(event Custom|ResetDirectionChangeCheck
  (Utilities|FlowControl|DoOnce false) ; enters at Reset
)

(event EventBeginPlay
  (Variables|Default|SetbMoveRight (Math|Random|RandomBool))
  (CallFunction|ToggleFacingDirection)
  (Rendering|SetVisibility (Variables|Default|GetStunned) false false))

(event EventTick
  (params (DeltaSeconds :type Float%20%28single-precision%29))
  (bind _bmoveright (Variables|Default|GetbMoveRight))
  (bind _stunned (Variables|Default|GetStunned))
  (if (Variables|Default|GetbCanMove)
    (Pawn|Input|AddMovementInput "1.000000, 0, 0" (select _bmoveright 1.0 -1.0) false)
    (if _bmoveright
      (Transformation|SetRelativeLocation _stunned "15.000000, 0,78.000000" false false)
      (else
        (Transformation|SetRelativeLocation _stunned "-15.000000, 0,78.000000" false false)))))

(fn ConstructionScript
  (|CallParentFunction))

(fn EnemyDied
  (|CallParentFunction)
  (bind _aswbp_text_points (Utilities|Casting|CastToWBP_TextPoints (UserInterface|GetUserWidgetObject (Variables|Default|GetPointText))))
  (Utilities|IsValid _aswbp_text_points
    (:Is%20Valid
      (Default|UpdatePointsDisplayed _aswbp_text_points (Utilities|Text|ToText(String) (Utilities|String|Append "+" (Utilities|String|ToString(Integer) (Variables|Default|GetPointsDelegated_0)))))
      (bind _asbp_player_base (Utilities|Casting|CastToBP_PlayerBase (Game|Player|GetPlayerPawn 0)))
      (Utilities|IsValid _asbp_player_base
        (:Is%20Valid
          (bind _output_get (Variables|/Script/Platformer.PlayerPaperCharacter|SetPoints _asbp_player_base (+ (Variables|/Script/Platformer.PlayerPaperCharacter|GetPoints _asbp_player_base) (Variables|Default|GetPointsDelegated_0))))
          (Default|UpdatePoints (Variables|/Game/Blueprints/Player/BP_PlayerBase.BP_PlayerBase_C|GetHUDRef _asbp_player_base) _output_get)
          (Collision|SetCollisionEnabled (Variables|Default|GetCapsuleComponent) "NoCollision")
          (Rendering|SetVisibility (Variables|Default|GetSprite) false false)
          (Game|SpawnActorfromClass "/Game/Blueprints/BP_SmokeEffect.BP_SmokeEffect_C" (Transformation|GetActorTransform) "AlwaysSpawn" 0 0)
          (Utilities|Time|SetTimerbyFunctionName 0 "DeathSequence" 2.0))))))

(fn ToggleFacingDirection
  (bind _sprite (Variables|Default|GetSprite))
  (bind _returnvalue (Transformation|GetWorldScale _sprite))
  (Transformation|SetWorldScale3D _sprite (Math|Vector|MakeVector (* (Math|Float|Absolute(Float) (.x _returnvalue)) (select (Variables|Default|GetbMoveRight) -1.0 1.0)) (.y _returnvalue) (.z _returnvalue))))

(fn DeathSequence
  (Actor|DestroyActor))