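; Side-scrolling sprite enemy that patrols along X, flipping at walls and at ledges found by a timed floor trace.
; An Attachment tracks the player and periodically traces for sight; detection permanently stops floor checks, starts looping projectile fire and eases the enemy toward the player while seen.
; A BP_Projectile overlap awards points to the player and HUD, hides the enemy with smoke and destroys it after a delay.
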(event OnComponentBeginOverlap(CapsuleComponent)
  (params (OverlappedComponent :type Primitive%20Component%20Object%20Reference) (OtherActor :type Actor%20Object%20Reference) (OtherComp :type Primitive%20Component%20Object%20Reference) (OtherBodyIndex :type Integer) (bFromSweep :type Boolean) (SweepResult :type Hit%20Result%20Structure%20%28by%20ref%29))
  (Utilities|Casting|CastToBP_Projectile OtherActor)
  (CallFunction|EnemyDied))

(event OnComponentHit(CapsuleComponent)
  (params (HitComponent :type Primitive%20Component%20Object%20Reference) (OtherActor :type Actor%20Object%20Reference) (OtherComp :type Primitive%20Component%20Object%20Reference) (NormalImpulse :type Vector :default "0, 0, 0") (Hit :type Hit%20Result%20Structure%20%28by%20ref%29))
  (if (!= OtherActor (Game|Player|GetPlayerPawn 0))
    (if (!= (.X (Math|Vector|BreakVector (.normal Hit))) 0.0)
      (Utilities|FlowControl|DoOnce false
        (:Completed
          (Variables|Default|SetbIsMovingRight (not (Variables|Default|GetbIsMovingRight)))
          (CallFunction|ToggleFacingDirection)
          (Utilities|FlowControl|Delay 0.2)
          (CallFunction|ResetDirectionChangeCheck))))))

(event Custom|ResetDirectionChangeCheck
  (Utilities|FlowControl|DoOnce false) ; enters at Reset
)

(event Custom|CheckIfThere'sFloor
  (CallFunction|FloorQuery))

(event Custom|TryDetectPlayer
  (bind _attachment (Variables|Default|GetAttachment))
  (bind _returnvalue (Transformation|GetWorldLocation _attachment))
  (bind _outhit (Collision|LineTraceByChannel _returnvalue (+ _returnvalue (* (Math|Vector|GetForwardVector _attachment) 1e+03)) "TraceTypeQuery1" false 0 "None" true "(R=1.000000,G=0.000000,B=0.000000,A=1.000000)" "(R=0.000000,G=1.000000,B=0.000000,A=1.000000)" 2.0))
  (bind _asbp_player_base (Utilities|Casting|CastToBP_PlayerBase (.hitactor _outhit))
    (:then
      (bind _output_get (Variables|Default|SetTarget _asbp_player_base))
      (if (< (.x (Transformation|GetActorLocation _output_get)) (.x (Transformation|GetActorLocation)))
        (Utilities|FlowControl|Delay 0.2)
        (Variables|Default|SetbIsMovingRight true)
        (CallFunction|ToggleFacingDirection)
        (else
          (Utilities|FlowControl|Delay 0.2)
          (Variables|Default|SetbIsMovingRight false)
          (CallFunction|ToggleFacingDirection)))
      (Utilities|Time|ClearandInvalidateTimerbyHandle (Variables|Default|GetCheckForFloorTimerHandle))
      (Utilities|FlowControl|DoOnce false
        (:Completed
          (Utilities|Time|SetTimerbyEvent (delegate Custom|ShootCd) 7.0 true))))
    (:CastFailed
      (Variables|Default|SetTarget 0))))

(event Custom|ShootCd
  (bind _attachment (Variables|Default|GetAttachment))
  (bind _returnvalue (Transformation|GetWorldTransform _attachment))
  (Game|SpawnActorfromClass "/Game/Blueprints/BP_EnemyShooterProjectile.BP_EnemyShooterProjectile_C" (Math|Transform|MakeTransform (.location _returnvalue) (.rotation _returnvalue) "1,1,1") "AlwaysSpawn" 0 0))

(event EventBeginPlay
  (bind _returnvalue (Actor|GetActorOfClass "/Game/Blueprints/Player/BP_PlayerBase.BP_PlayerBase_C"))
  (Variables|Default|SetPlayerRef _returnvalue)
  (Variables|Default|SetbIsMovingRight (Math|Random|RandomBool))
  (CallFunction|ToggleFacingDirection)
  (bind _returnvalue_2 (Utilities|Time|SetTimerbyEvent (delegate Custom|CheckIfThere'sFloor) 0.2 true))
  (Variables|Default|SetCheckForFloorTimerHandle _returnvalue_2)
  (Utilities|Time|SetTimerbyEvent (delegate Custom|TryDetectPlayer) 2.0 true))

(event EventEnemyDied
  (bind _aswbp_text_points (Utilities|Casting|CastToWBP_TextPoints (UserInterface|GetUserWidgetObject (Variables|Default|GetPointText))))
  (Utilities|IsValid _aswbp_text_points
    (:Is%20Valid
      (Default|UpdatePointsDisplayed _aswbp_text_points (Utilities|Text|ToText(String) (Utilities|String|Append "+" (Utilities|String|ToString(Integer) (Variables|Default|GetPointsDelegated)))))
      (bind _asbp_player_base (Utilities|Casting|CastToBP_PlayerBase (Game|Player|GetPlayerPawn 0)))
      (Utilities|IsValid _asbp_player_base
        (:Is%20Valid
          (bind _output_get (Variables|/Script/Platformer.PlayerPaperCharacter|SetPoints _asbp_player_base (+ (Variables|/Script/Platformer.PlayerPaperCharacter|GetPoints _asbp_player_base) (Variables|Default|GetPointsDelegated))))
          (Default|UpdatePoints (Variables|/Game/Blueprints/Player/BP_PlayerBase.BP_PlayerBase_C|GetHUDRef _asbp_player_base) _output_get)
          (Collision|SetCollisionEnabled (Variables|Default|GetCapsuleComponent) "NoCollision")
          (Rendering|SetVisibility (Variables|Default|GetSprite) false false)
          (Game|SpawnActorfromClass "/Game/Blueprints/BP_SmokeEffect.BP_SmokeEffect_C" (Transformation|GetActorTransform) "AlwaysSpawn" 0 0)
          (Utilities|Time|SetTimerbyFunctionName 0 "DeathSequence" 2.0))))))

(event EventTick
  (params (DeltaSeconds :type Float%20%28single-precision%29))
  (bind _bismovingright (Variables|Default|GetbIsMovingRight))
  (bind _detectionpoint (Variables|Default|GetDetectionPoint))
  (bind _playerref (Variables|Default|GetPlayerRef))
  (bind _attachment (Variables|Default|GetAttachment))
  (Utilities|IsValid _playerref
    (:Is%20Valid
      (Transformation|SetWorldRotation _attachment (Math|Rotator|FindLookatRotation (Transformation|GetWorldLocation _attachment) (Transformation|GetActorLocation _playerref)) false false)
      (if (Utilities|IsValid (Variables|Default|GetTarget))
        (Transformation|SetActorLocation (Math|Interpolation|VInterpTo (Transformation|GetActorLocation) (Transformation|GetActorLocation (Variables|Default|GetTarget)) (Utilities|Time|GetWorldDeltaSeconds) 0.15) false false)
        (else
          (Pawn|Input|AddMovementInput "1.000000, 0, 0" (Math|Float|SelectFloat -1.0 1.0 _bismovingright) false)
          (if _bismovingright
            (Transformation|SetRelativeLocation _detectionpoint "-57.000000, 0, 0" false false)
            (else
              (Transformation|SetRelativeLocation _detectionpoint "57.000000, 0, 0" false false))))))))

(fn ConstructionScript
  (|CallParentFunction))

(fn ToggleFacingDirection
  (bind _sprite (Variables|Default|GetSprite))
  (bind _returnvalue (Transformation|GetWorldScale _sprite))
  (Transformation|SetWorldScale3D _sprite (Math|Vector|MakeVector (* (Math|Float|Absolute(Float) (.x _returnvalue)) (select (Variables|Default|GetbIsMovingRight) 1.0 -1.0)) (.y _returnvalue) (.z _returnvalue))))

(fn FloorQuery
  (bind _detectionpoint (Variables|Default|GetDetectionPoint))
  (bind _returnvalue (Transformation|GetWorldLocation _detectionpoint))
  (bind _returnvalue_2 (Collision|LineTraceByChannel _returnvalue (+ _returnvalue (* (Math|Vector|GetUpVector _detectionpoint) -1.5e+02)) "TraceTypeQuery1" false 0 "None" true "(R=1.000000,G=0.000000,B=0.000000,A=1.000000)" "(R=0.000000,G=1.000000,B=0.000000,A=1.000000)" 2.0))
  (if (not _returnvalue_2)
    (Variables|Default|SetbIsMovingRight (not (Variables|Default|GetbIsMovingRight)))
    (CallFunction|ToggleFacingDirection)))

(fn DeathSequence
  (Actor|DestroyActor))