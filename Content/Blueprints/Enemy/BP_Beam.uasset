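; BP_Beam is a turret enemy that slows or damages players caught in its forward beam via TakeSlowDamage.
; A looping timer runs a visibility line trace from LilCube along its forward vector, with a debug line drawn for each trace.
; Once IsDead is set, the next tick clears the timer, spawns smoke and moves the non-looping TurretFB playback from midpoint to a later position.
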(event Custom|ApplyBeam
  (bind _lilcube (Variables|Default|GetLilCube))
  (bind _returnvalue (Transformation|GetWorldLocation _lilcube))
  (bind _outhit (Collision|LineTraceByChannel _returnvalue (+ _returnvalue (* (Math|Vector|GetForwardVector (Transformation|GetWorldRotation _lilcube)) (Variables|Default|GetTraceDistance))) "TraceTypeQuery1" false 0 "ForDuration" true "(R=1.000000,G=0.000000,B=0.000000,A=1.000000)" "(R=0.000000,G=1.000000,B=0.000000,A=0.000000)" 0.1))
  (if (Variables|Default|GetIsDead)
    (Utilities|Time|ClearandInvalidateTimerbyHandle (Variables|Default|GetBeamTimerHandle))
    (CallFunction|EnemyDied)
    (else
      (bind _asbp_player_base (Utilities|Casting|CastToBP_PlayerBase (.hitactor _outhit)))
      (Default|TakeSlowDamage _asbp_player_base self))))

(event EventBeginPlay
  (bind _turretfb (Variables|Default|GetTurretFB))
  (Components|Timeline|SetLooping _turretfb false)
  (Components|Timeline|SetPlaybackPosition _turretfb 0.5 false)
  (bind _returnvalue (Utilities|Time|SetTimerbyEvent (delegate Custom|ApplyBeam) 0.1 true))
  (Variables|Default|SetBeamTimerHandle _returnvalue))

(fn ConstructionScript
  (|CallParentFunction))

(fn EnemyDied
  (bind _returnvalue (Transformation|GetActorLocation))
  (|CallParentFunction)
  (Game|SpawnActorfromClass "/Game/Blueprints/BP_SmokeEffect.BP_SmokeEffect_C" (Math|Transform|MakeTransform (Math|Vector|MakeVector (+ (.x _returnvalue) 26.0) (.y _returnvalue) (+ (.z _returnvalue) 45.0)) "0, 0, 0" "1,1,1") "AlwaysSpawn" 0 0)
  (Components|Timeline|SetPlaybackPosition (Variables|Default|GetTurretFB) 1.0 false))