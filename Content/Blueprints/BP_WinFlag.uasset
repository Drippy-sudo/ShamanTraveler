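; BP_WinFlag is a level goal actor that triggers the win sequence when a BP_PlayerBase overlaps its WinCollider.
; On the first overlap it clears all widgets, shows WBP_WinScreen, flags player movement to stop and starts a looping one-second timer.
; Tick then disables CanMove once on the controlled pawn.
; The timer updates the on-screen countdown and restarts the level via console command when it runs out.
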(event OnComponentBeginOverlap(WinCollider)
  (params (OverlappedComponent :type Primitive%20Component%20Object%20Reference) (OtherActor :type Actor%20Object%20Reference) (OtherComp :type Primitive%20Component%20Object%20Reference) (OtherBodyIndex :type Integer) (bFromSweep :type Boolean) (SweepResult :type Hit%20Result%20Structure%20%28by%20ref%29))
  ;[1 1 1] Win cycle
  (bind _asbp_player_base (Utilities|Casting|CastToBP_PlayerBase OtherActor))
  (Utilities|FlowControl|DoOnce false
    (:Completed
      (Viewport|RemoveAllWidgets)
      (bind _asbp_player_controller (Utilities|Casting|CastToBP_PlayerController (Pawn|GetController _asbp_player_base)))
      (bind _returnvalue (UserInterface|CreateWidget "/Game/Assets/Widgets/WBP_WinScreen.WBP_WinScreen_C" _asbp_player_controller))
      (bind _output_get (Variables|Default|SetWinWidget _returnvalue))
      (Default|UpdateCountdownText _output_get (Variables|Default|GetCountdown))
      (UserInterface|Viewport|AddtoViewport _output_get 0)
      (Variables|Default|SetShouldStopPlayerMovement true)
      (Utilities|Time|SetTimerbyEvent (delegate Custom|ReduceCountdown) 1.0 true))))

(event Custom|ReduceCountdown
  ;[1 1 1] Win cycle
  (if (<= (Variables|Default|GetCountdown) 0)
    (Development|ExecuteConsoleCommand "RestartLevel" 0)
    (else
      (bind _result (Math|Integer|DecrementInt (Variables|Default|GetCountdown))
        (:%20%20
          (bind _output_get (Variables|Default|SetCountdown _result))
          (Default|UpdateCountdownText (Variables|Default|GetWinWidget) _output_get))))))

(event EventBeginPlay)

(event Collision|EventActorBeginOverlap
  (params (OtherActor :type Actor%20Object%20Reference)))

(event EventTick
  (params (DeltaSeconds :type Float%20%28single-precision%29))
  ;[1 1 1] Stop player movement
  (if (Variables|Default|GetShouldStopPlayerMovement)
    (Utilities|FlowControl|DoOnce false
      (:Completed
        (bind _asbp_player_base (Utilities|Casting|CastToBP_PlayerBase (Pawn|GetControlledPawn (Game|GetPlayerController 0))))
        (Variables|/Script/Platformer.PlayerPaperCharacter|SetCanMove _asbp_player_base false)))))

(fn ConstructionScript)