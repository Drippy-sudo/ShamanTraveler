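; BP_DeathZone is a trigger volume that kills the player with a short countdown, then respawns them at their checkpoint.
; On overlap it detaches the camera in place, shows a restart counter widget and runs a looping DeathProcess timer, with DoOnce gates re-armed on end overlap.
; Respawn teleports the player and restores health, or restarts the level without a checkpoint.
; With enough points, it also halves them, spawns smoke and schedules camera reattachment.
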(event OnComponentBeginOverlap(Box)
  (params (OverlappedComponent :type Primitive%20Component%20Object%20Reference) (OtherActor :type Actor%20Object%20Reference) (OtherComp :type Primitive%20Component%20Object%20Reference) (OtherBodyIndex :type Integer) (bFromSweep :type Boolean) (SweepResult :type Hit%20Result%20Structure%20%28by%20ref%29))
  (Variables|Default|SetCountDown 2)
  (bind _asbp_player_base (Utilities|Casting|CastToBP_PlayerBase OtherActor))
  (bind _output_get (Variables|Default|SetPlayerRef _asbp_player_base))
  (Variables|Default|SetPlayerSpawnLocation (Variables|/Game/Blueprints/Player/BP_PlayerBase.BP_PlayerBase_C|GetSpawnLocation _output_get))
  (Transformation|DetachFromComponent (Variables|/Game/Blueprints/Player/BP_PlayerBase.BP_PlayerBase_C|GetCamera (Variables|Default|GetPlayerRef)) "KeepWorld" "KeepWorld" "KeepWorld" true)
  (Variables|Default|SetCameraLastLocation (Transformation|GetWorldLocation (Variables|/Game/Blueprints/Player/BP_PlayerBase.BP_PlayerBase_C|GetCamera (Variables|Default|GetPlayerRef))))
  (Transformation|SetWorldLocation (Variables|/Game/Blueprints/Player/BP_PlayerBase.BP_PlayerBase_C|GetCamera (Variables|Default|GetPlayerRef)) (Variables|Default|GetCameraLastLocation) false false)
  (Utilities|FlowControl|DoOnce false
    (:Completed
      (Viewport|RemoveAllWidgets)
      (bind _asbp_player_controller (Utilities|Casting|CastToBP_PlayerController (Pawn|GetController (Variables|Default|GetPlayerRef))))
      (bind _output_get_2 (Variables|Default|SetPlayerControllerRef _asbp_player_controller))
      (bind _returnvalue (UserInterface|CreateWidget "/Game/Assets/Widgets/WBP_RestartCounter.WBP_RestartCounter_C" _output_get_2))
      (bind _output_get_3 (Variables|Default|SetCountdownWidget _returnvalue))
      (Default|UpdateCountdownText _output_get_3 (Variables|Default|GetCountDown))
      (UserInterface|Viewport|AddtoPlayerScreen _output_get_3)
      (bind _returnvalue_2 (Utilities|Time|SetTimerbyFunctionName 0 "DeathProcess" 1.0 true))
      (Variables|Default|SetDeathCycleTimerHandle _returnvalue_2))))

(event OnComponentEndOverlap(Box)
  (params (OverlappedComponent :type Primitive%20Component%20Object%20Reference) (OtherActor :type Actor%20Object%20Reference) (OtherComp :type Primitive%20Component%20Object%20Reference) (OtherBodyIndex :type Integer))
  (Utilities|Casting|CastToBP_PlayerBase OtherActor)
  (Utilities|FlowControl|DoOnce false
    (:Completed
      (bind _output_get (Variables|Default|SetCountDown 2))
      (Default|UpdateCountdownText (Variables|Default|GetCountdownWidget) _output_get)
      (CallFunction|RestartDeathCycle))))

(event Custom|RestartDeathCycle
  (CallFunction|ResetEndOverlap)
  (Utilities|FlowControl|DoOnce false) ; enters at Reset
)

(event Custom|Reset%20End%20Overlap
  (Utilities|FlowControl|DoOnce false) ; enters at Reset
)

(event Collision|EventActorBeginOverlap
  (params (OtherActor :type Actor%20Object%20Reference)))

(fn ConstructionScript)

(fn RespawnPlayer
  (params (Player :type BP%20Player%20Base%20Object%20Reference))
  (bind _playerref (Variables|Default|GetPlayerRef))
  (bind _playerref_2 (Variables|Default|GetPlayerRef))
  (bind _playerref_3 (Variables|Default|GetPlayerRef))
  (bind _playerref_4 (Variables|Default|GetPlayerRef))
  (bind _playerref_5 (Variables|Default|GetPlayerRef))
  (bind _returnvalue (Transformation|GetActorLocation _playerref_4))
  (if (Class|KismetMathLibrary|EqualExactlyVectorVector (Variables|/Game/Blueprints/Player/BP_PlayerBase.BP_PlayerBase_C|GetCheckpointLocation (Variables|Default|GetPlayerRef)) "0, 0, 0")
    (Development|ExecuteConsoleCommand "RestartLevel" (Game|GetPlayerController 0) :!label _label)
    (else
      (Utilities|IsValid (Variables|Default|GetPlayerRef)
        (:Is%20Valid
          (Transformation|SetActorLocation _playerref_2 (Variables|/Game/Blueprints/Player/BP_PlayerBase.BP_PlayerBase_C|GetCheckpointLocation _playerref_2) false false)
          (Transformation|SetActorRelativeRotation "0, 0, 0")
          (Default|RemoveSelf (Variables|Default|GetCountdownWidget))
          (Default|RespawnWidgets _playerref_5)
          (bind _output_get (Variables|/Game/Blueprints/Player/BP_PlayerBase.BP_PlayerBase_C|SetHealth _playerref_5 (Variables|/Game/Blueprints/Player/BP_PlayerBase.BP_PlayerBase_C|GetDefaultHealth _playerref_5)))
          (Default|UpdateHealth (Variables|/Game/Blueprints/Player/BP_PlayerBase.BP_PlayerBase_C|GetHUDRef _playerref) _output_get)
          (if (>= (Variables|/Script/Platformer.PlayerPaperCharacter|GetPoints _playerref) 2)
            (bind _output_get_2 (Variables|/Script/Platformer.PlayerPaperCharacter|SetPoints _playerref_3 (/ (Variables|/Script/Platformer.PlayerPaperCharacter|GetPoints _playerref) 2)))
            (Default|UpdatePoints (Variables|/Game/Blueprints/Player/BP_PlayerBase.BP_PlayerBase_C|GetHUDRef _playerref_3) _output_get_2)
            (Utilities|Time|SetTimerbyFunctionName 0 "MoveCamera" 0.2)
            (Game|SpawnActorfromClass "/Game/Blueprints/BP_SmokeEffect.BP_SmokeEffect_C" (Math|Transform|MakeTransform (Math|Vector|MakeVector (.x _returnvalue) (- (.y _returnvalue) 1.0) (.z _returnvalue)) "0, 0, 0" "1,1,1") "AlwaysSpawn" 0 0)))
        (:Is%20Not%20Valid
          (goto _label))))))

(fn DeathProcess
  (bind _result (Math|Integer|DecrementInt (Variables|Default|GetCountDown))
    (:%20%20
      (bind _output_get (Variables|Default|SetCountDown _result))
      (Default|UpdateCountdownText (Variables|Default|GetCountdownWidget) _output_get)
      (if (<= (Variables|Default|GetCountDown) 0)
        (CallFunction|RespawnPlayer (Variables|Default|GetPlayerRef))
        (Utilities|Time|ClearandInvalidateTimerbyHandle (Variables|Default|GetDeathCycleTimerHandle))))))

(fn MoveCamera
  (bind _playerref (Variables|Default|GetPlayerRef))
  (Transformation|AttachComponentToComponent (Variables|/Game/Blueprints/Player/BP_PlayerBase.BP_PlayerBase_C|GetCamera _playerref) (Variables|/Game/Blueprints/Player/BP_PlayerBase.BP_PlayerBase_C|GetSpringArm _playerref) "None" "SnapToTarget" "SnapToTarget" "SnapToTarget" true)
  (Default|RemoveSelf (Variables|Default|GetCountdownWidget)))