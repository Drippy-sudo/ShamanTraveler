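; BP_MovingTerrain is a moving terrain piece that starts moving with an elevator sound once its assigned target is hit.
; Tick polls BPTarget.WasHit and, through a DoOnce, sets CanMove, spawns the attenuated sound and starts a looping timer that moves it to the actor's location.
; The movement itself is not in these graphs; the ReachedDestination event stops the sound after a short delay.
; A missing target prints a warning every tick.
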(event Custom|SetSoundLocation
  (Utilities|IsValid (stale EventTick _output_get)
    (:Is%20Valid
      (Transformation|SetWorldLocation (stale EventTick _output_get) (Transformation|GetActorLocation) false false))))

(event EventReachedDestination
  (Utilities|IsValid (stale EventTick _output_get)
    (:Is%20Valid
      (Utilities|FlowControl|Delay 0.2)
      (Audio|Components|Audio|Stop (stale EventTick _output_get)))))

(event EventTick
  (params (DeltaSeconds :type Float%20%28single-precision%29))
  (bind _bp_target (Variables|Default|GetBP_Target))
  (Utilities|IsValid _bp_target
    (:Is%20Valid
      (if (Variables|/Game/Blueprints/SmartTerrain/BP_Target.BP_Target_C|GetWasHit _bp_target)
        (Utilities|FlowControl|DoOnce false
          (:Completed
            (Variables|Default|SetCanMove true)
            (bind _returnvalue (Audio|SpawnSoundatLocation "/Game/Assets/Sounds/Elevator.Elevator" (Transformation|GetActorLocation) "0, 0, 0" 1.0 0.5 0.0 "/Game/BasicAttenuation.BasicAttenuation" 0))
            (bind _output_get (Variables|Default|SetEleSound _returnvalue))
            (Utilities|Time|SetTimerbyEvent (delegate Custom|SetSoundLocation) 1.0 true)))))
    (:Is%20Not%20Valid
      (Development|PrintString "Please Select A Target For A Moving Terrain"))))

(fn ConstructionScript)