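; BP_Target is a hittable target with a Totem flipbook that reacts to projectiles.
; A BP_Projectile overlapping its Box sets WasHit and sets the flipbook play rate to normal speed.
; Looping is disabled at BeginPlay, and when playback finishes the flipbook is moved to its end frame without firing events, leaving the totem in its final state.
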(event OnFinishedPlaying(Totem)
  (bind _totem (Variables|Default|GetTotem))
  (Class|PaperFlipbookComponent|SetPlaybackPositioninFrames _totem (Class|PaperFlipbookComponent|GetFlipbookLengthinFrames _totem) false)
  (Components|Timeline|SetLooping _totem false))

(event OnComponentBeginOverlap(Box)
  (params (OverlappedComponent :type Primitive%20Component%20Object%20Reference) (OtherActor :type Actor%20Object%20Reference) (OtherComp :type Primitive%20Component%20Object%20Reference) (OtherBodyIndex :type Integer) (bFromSweep :type Boolean) (SweepResult :type Hit%20Result%20Structure%20%28by%20ref%29))
  (Utilities|Casting|CastToBP_Projectile OtherActor)
  (Variables|Default|SetWasHit true)
  (Components|Timeline|SetPlayRate (Variables|Default|GetTotem) 1.0))

(event EventBeginPlay
  (Components|Timeline|SetLooping (Variables|Default|GetTotem) false))

(event Collision|EventActorBeginOverlap
  (params (OtherActor :type Actor%20Object%20Reference)))

(event EventTick
  (params (DeltaSeconds :type Float%20%28single-precision%29)))

(fn ConstructionScript)