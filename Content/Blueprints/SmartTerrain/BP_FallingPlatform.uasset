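; BP_FallingPlatform is a smart terrain platform that drops after a player touches it and later removes itself.
; When a BP_PlayerBase overlaps the Box trigger, two timers start.
; After TimeBeforeFall the StaticMesh switches to a PhysicsBody object type and simulates physics, and after TimeBeforeDeletion the actor is destroyed.
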(event OnComponentBeginOverlap(Box)
  (params (OverlappedComponent :type Primitive%20Component%20Object%20Reference) (OtherActor :type Actor%20Object%20Reference) (OtherComp :type Primitive%20Component%20Object%20Reference) (OtherBodyIndex :type Integer) (bFromSweep :type Boolean) (SweepResult :type Hit%20Result%20Structure%20%28by%20ref%29))
  (Utilities|Casting|CastToBP_PlayerBase OtherActor)
  (Utilities|Time|SetTimerbyEvent (delegate Custom|SetActorToPhysicsActor) (Variables|Default|GetTimeBeforeFall))
  (Utilities|Time|SetTimerbyEvent (delegate Custom|DeleteActor) (Variables|Default|GetTimeBeforeDeletion)))

(event Custom|DeleteActor
  (Actor|DestroyActor))

(event Custom|SetActorToPhysicsActor
  (Collision|SetCollisionObjectType (Variables|Default|GetStaticMesh) "ECC_PhysicsBody")
  (Physics|SetSimulatePhysics (Variables|Default|GetStaticMesh) true))

(fn ConstructionScript)