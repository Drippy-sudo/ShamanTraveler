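; Liftable smart-terrain physics object that crushes players and enemies it overlaps while in slow-fall mode.
; Tick raises the mesh's mass scale once when it simulates physics in that mode.
; ResetPhysics overlaps call HitableActorHit, which damages the victim, disables its collision, hides it and spawns smoke.
; The RockFB flipbook freezes on finishing and turns off mesh collision; a separate event disables all three collision components.
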(event OnComponentBeginOverlap(ResetPhysics)
  (params (OverlappedComponent :type Primitive%20Component%20Object%20Reference) (OtherActor :type Actor%20Object%20Reference) (OtherComp :type Primitive%20Component%20Object%20Reference) (OtherBodyIndex :type Integer) (bFromSweep :type Boolean) (SweepResult :type Hit%20Result%20Structure%20%28by%20ref%29))
  (Utilities|Casting|CastToBP_Mana OtherActor
    (:CastFailed
      (if (Variables|Default|GetbIsInSlowFallMode)
        (bind _asbp_enemy_base (Utilities|Casting|CastToBP_EnemyBase OtherActor)
          (:then
            (bind _output_get (Variables|Default|SetEnemyRef _asbp_enemy_base))
            (CallFunction|HitableActorHit _output_get))
          (:CastFailed
            (bind _asbp_player_base (Utilities|Casting|CastToBP_PlayerBase OtherActor))
            (Variables|Default|SetPlayerRef _asbp_player_base)
            (CallFunction|HitableActorHit (Variables|Default|GetPlayerRef))))))))

(event OnComponentEndOverlap(ResetPhysics)
  (params (OverlappedComponent :type Primitive%20Component%20Object%20Reference) (OtherActor :type Actor%20Object%20Reference) (OtherComp :type Primitive%20Component%20Object%20Reference) (OtherBodyIndex :type Integer))
  (Utilities|Casting|CastToBP_EnemyBase OtherActor
    (:CastFailed
      (Utilities|Casting|CastToBP_PlayerBase OtherActor))))

(event OnFinishedPlaying(RockFB)
  (bind _rockfb (Variables|Default|GetRockFB))
  (Components|Timeline|SetPlaybackPosition _rockfb 1.0 false)
  (Components|Timeline|SetPlayRate _rockfb 0.0)
  (Collision|SetCollisionEnabled (Variables|Default|GetStaticMeshComp) "NoCollision"))

(event Custom|SetCollisionOff
  (Collision|SetCollisionEnabled (Variables|Default|GetStaticMeshComp) "NoCollision")
  (Collision|SetCollisionEnabled (Variables|Default|GetResetPhysics) "NoCollision")
  (Collision|SetCollisionEnabled (Variables|Default|GetBoxComp) "NoCollision"))

(event EventBeginPlay
  (Components|Timeline|SetLooping (Variables|Default|GetRockFB) false))

(event EventTick
  (params (DeltaSeconds :type Float%20%28single-precision%29))
  (if (and (Physics|IsSimulatingPhysics (Variables|Default|GetStaticMeshComp) "None") (Variables|Default|GetbIsInSlowFallMode))
    (Utilities|FlowControl|DoOnce false
      (:Completed
        (Class|PrimitiveComponent|SetMassScale (Variables|Default|GetStaticMeshComp) "None" 1.5e+02)))))

(fn ConstructionScript)

(fn HitableActorHit
  (params (Actor :type Actor%20Object%20Reference))
  (Collision|SetActorEnableCollision Actor false)
  (Game|Damage|ApplyDamage Actor 1e+02 0 0)
  (Rendering|SetActorHiddenInGame Actor true)
  (Game|SpawnActorfromClass "/Game/Blueprints/BP_SmokeEffect.BP_SmokeEffect_C" (Transformation|GetActorTransform Actor) "AlwaysSpawn" 0 0))