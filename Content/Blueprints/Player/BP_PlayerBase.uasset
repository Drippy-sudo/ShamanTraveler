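; Base player character for a 2D flipbook side-scroller with HUD, health, wall jumping and a charged spell shot.
; Tick flips sprite, wall collider and fire point by velocity, and polls shooting, which slows movement while charging before firing a child BP_Shooter.
; Landing on enemies kills them and bounces the player; other enemy hits cause damage and knockback.
; Death detaches the camera, rotates the body and runs a countdown before restarting the level.
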(event OnComponentHit(CapsuleComponent)
  (params (HitComponent :type Primitive%20Component%20Object%20Reference) (OtherActor :type Actor%20Object%20Reference) (OtherComp :type Primitive%20Component%20Object%20Reference) (NormalImpulse :type Vector :default "0, 0, 0") (Hit :type Hit%20Result%20Structure%20%28by%20ref%29))
  (bind _charactermovement (Variables|Character|GetCharacterMovement))
  (bind _asbp_enemy_base (Utilities|Casting|CastToBP_EnemyBase OtherActor))
  (Variables|Default|SetHitEnemy _asbp_enemy_base)
  (Utilities|FlowControl|DoOnce false
    (:Completed
      (Variables|Default|SetHitDirection (Math|Vector|Normalize (- (.location Hit) (Transformation|GetActorLocation)) 0.0))
      (Utilities|FlowControl|Sequence
        (:then_0
          (if (<= (.z (Variables|Default|GetHitDirection)) -0.1)
            ;[1 1 1] Damage enemy
            (Variables|/Script/Engine.MovementComponent|SetVelocity _charactermovement "0, 0, 0")
            (Components|Movement|StopMovementImmediately _charactermovement)
            (Physics|AddImpulse _charactermovement (Math|Vector|MakeVector 0.0 0.0 (Variables|Default|GetEnemyHitKnockBackForce)) true)
            (Game|Damage|ApplyDamage (Variables|Default|GetHitEnemy) (Variables|/Game/Blueprints/Enemy/BP_EnemyBase.BP_EnemyBase_C|GetHealth (Variables|Default|GetHitEnemy)) 0 0)
            (else
              ;[1 1 1] Damage Player
              (Variables|/Script/Engine.MovementComponent|SetVelocity _charactermovement "0, 0, 0")
              (Components|Movement|StopMovementImmediately _charactermovement)
              (Physics|AddImpulse _charactermovement (Math|Vector|MakeVector (* (.x (Variables|Default|GetHitDirection)) (* -1.0 (Variables|Default|GetTakeDmgKnockBackForce))) 0.0 (Variables|Default|GetZHeightTakeDmgKnockBack)) true)
              (Game|Damage|ApplyDamage self (Variables|Default|GetBase%20Damage) 0 0))))
        (:then_1
          (Utilities|FlowControl|Delay 0.1)
          (CallFunction|ResetDamageImpulse))))))

(event OnComponentBeginOverlap(WallCollider)
  (params (OverlappedComponent :type Primitive%20Component%20Object%20Reference) (OtherActor :type Actor%20Object%20Reference) (OtherComp :type Primitive%20Component%20Object%20Reference) (OtherBodyIndex :type Integer) (bFromSweep :type Boolean) (SweepResult :type Hit%20Result%20Structure%20%28by%20ref%29))
  ;[1 1 1] Handles wall jumping
  (Utilities|FlowControl|DoOnce false
    (:Completed
      (Utilities|Casting|CastToBP_EnemyBat OtherActor
        (:CastFailed
          (Variables|Default|SetIsTouchingFront true)
          (Utilities|FlowControl|Delay 0.2)
          (if (Variables|Default|GetIsTouchingFront)
            (if (Variables|Default|GetHasLeftWall)
              (bind _result (Math|Integer|IncrementInt (Variables|Default|GetJump%20Max%20Count%20Num))
                (:%20%20
                  (Variables|Default|SetJumpMaxCount _result))))))))))

(event OnComponentEndOverlap(WallCollider)
  (params (OverlappedComponent :type Primitive%20Component%20Object%20Reference) (OtherActor :type Actor%20Object%20Reference) (OtherComp :type Primitive%20Component%20Object%20Reference) (OtherBodyIndex :type Integer))
  ;[1 1 1] Handles wall jumping
  (Utilities|FlowControl|Sequence
    (:then_0
      (Variables|Default|SetIsJumping false)
      (Variables|Default|SetIsJumping true)
      (Variables|Default|SetHasLeftWall true)
      (Utilities|FlowControl|Delay 0.1)
      (Variables|Default|SetJumpMaxCount 1)
      (if (Variables|Default|GetIsTouchingFront)
        (Utilities|FlowControl|Delay 0.1)
        (Variables|Default|SetIsTouchingFront false)))
    (:then_1
      (Utilities|FlowControl|DoOnce false) ; enters at Reset
    )))

(event Custom|ResetDamageImpulse
  (bind _charactermovement (Variables|Character|GetCharacterMovement))
  (bind _hitenemy (Variables|Default|GetHitEnemy))
  (Utilities|FlowControl|DoOnce false) ; enters at Reset
)

(event Custom|ShootCall
  (bind _over9000 (Variables|Default|GetOver9000))
  (bind _over9000_2 (Variables|Default|GetOver9000))
  ;[1 1 1] Shoots
  (if (Utilities|TestifCanShoot)
    (Components|Timeline|SetPlaybackPosition (Variables|Default|GetOver9000) 0.0 false)
    (Variables|/Script/Engine.CharacterMovementComponent|SetMaxWalkSpeed (Variables|Character|GetCharacterMovement) 3e+02)
    (Variables|Default|SetSpellChargeCounter (+ (Variables|Default|GetSpellChargeCounter) 0.1))
    (Components|Timeline|SetPlaybackPosition _over9000 (- (+ (Variables|Default|GetSpellChargeCounter) 0.1) 0.001) false)
    (Rendering|SetVisibility _over9000 true false)
    (Components|Timeline|SetPlayRate _over9000 1.0)
    (if (>= (Variables|Default|GetSpellChargeCounter) (Variables|Default|GetSpellChargeCounterMax))
      (Variables|Default|SetSpellChargeCounter 0.0)
      (bind _asbp_shooter (Utilities|Casting|CastToBP_Shooter (Variables|/Script/Engine.ChildActorComponent|GetChildActor (Variables|Default|GetChildActor))))
      (Default|Fire _asbp_shooter)
      (Variables|Default|SetCanShoot false)
      (Utilities|FlowControl|DoOnce false
        (:Completed
          (bind _returnvalue (Utilities|Time|SetTimerbyEvent (delegate Custom|ResetFireCD) (Variables|Default|GetShootCD) true))
          (Variables|Default|SetShootTimerHandle _returnvalue))))
    (else
      (Variables|Default|SetSpellChargeCounter 0.0)
      (Variables|/Script/Engine.CharacterMovementComponent|SetMaxWalkSpeed (Variables|Character|GetCharacterMovement) 6e+02)
      (Rendering|SetVisibility _over9000_2 false false)
      (Components|Timeline|SetPlayRate _over9000_2 0.0)
      (Components|Timeline|SetPlaybackPosition _over9000_2 0.0 false))))

(event Custom|ResetFireCD
  ;[1 1 1] Shoots
  (Variables|Default|SetCanShoot true))

(event EventBeginPlay
  ;[1 1 1] Creates widgets
  (|CallParentFunction)
  (Components|Timeline|SetLooping (Variables|Default|GetOver9000) false)
  (Rendering|SetVisibility (Variables|Default|GetSprite) true false)
  (Variables|Default|SetIsDead false)
  (Variables|Default|SetSpawnLocation (Transformation|GetActorLocation))
  (bind _returnvalue (UserInterface|CreateWidget "/Game/Assets/Widgets/WBP_HUD.WBP_HUD_C" (Game|GetPlayerController 0)))
  (bind _output_get (Variables|Default|SetHUDRef _returnvalue))
  (UserInterface|Viewport|AddtoViewport _output_get 0)
  (Default|UpdatePoints (Variables|Default|GetHUDRef)))

(event EventTick
  (params (DeltaSeconds :type Float%20%28single-precision%29))
  (bind _firepoint (Variables|Default|GetFirePoint))
  (bind _wallcollider (Variables|Default|GetWallCollider))
  ;[1 1 1] Handles player rotation
  (|CallParentFunction DeltaSeconds)
  (if (Variables|Default|GetShouldRotate)
    ;[1 1 1] Death animation
    (Transformation|SetActorRelativeRotation (Math|Rotator|Lerp(Rotator) (Transformation|GetActorRotation) "90.000000, 0, 0" (* (Utilities|Time|GetWorldDeltaSeconds) (Variables|Default|GetDeathRotateSpeed))))
    (Components|Timeline|SetPlayRate (Variables|Default|GetSprite) 0.0)
    (else
      (CallFunction|ShootCall)
      (Math|Float|CompareFloat (.x (Variables|/Script/Engine.MovementComponent|GetVelocity (Variables|Character|GetCharacterMovement))) 0.0
        (:>
          (Transformation|SetRelativeRotation (Variables|Default|GetSprite) (Math|Rotator|MakeRotator 0.0 0.0 0.0) false false)
          (Transformation|SetRelativeLocation _wallcollider "50.000000, 0, 0" false false)
          (Transformation|SetRelativeLocation _firepoint "84.000000, 0, 0" false false)
          (Transformation|SetRelativeRotation _firepoint "0, 0, 0" false false))
        (:<
          (Transformation|SetRelativeRotation (Variables|Default|GetSprite) (Math|Rotator|MakeRotator 0.0 0.0 1.8e+02) false false)
          (Transformation|SetRelativeLocation _wallcollider "-50.000000, 0, 0" false false)
          (Transformation|SetRelativeLocation _firepoint "-84.000000, 0, 0" false false)
          (Transformation|SetRelativeRotation _firepoint "0,180.000000,0.000000" false false))))))

(event EventOnLanded
  (params (Hit :type Hit%20Result%20Structure%20%28by%20ref%29))
  ;[1 1 1] On Landed sets max jump count
  (if (.bBlockingHit (Collision|BreakHitResult Hit))
    (Variables|Default|SetJump%20Max%20Count%20Num 1)))

(event Game|Damage|EventAnyDamage
  (params (Damage :type Float%20%28single-precision%29) (DamageType :type Damage%20Type%20Object%20Reference) (InstigatedBy :type Controller%20Object%20Reference) (DamageCauser :type Actor%20Object%20Reference))
  ;[1 1 1] Handle Damage
  (bind _output_get (Variables|Default|SetHealth (Math|Float|Clamp(Float) (- (Variables|Default|GetHealth) Damage) 0.0 (Variables|Default|GetDefaultHealth))))
  ;[1 1 1] Handle Death
  (Default|UpdateHealth (Variables|Default|GetHUDRef) _output_get)
  (if (and (<= (Variables|Default|GetHealth) 0.0) (not (Variables|Default|GetIsDead)))
    (Variables|Default|SetIsDead true)
    (CallFunction|Death)))

(event EventUpdateRunningAnimation
  ;[1 1 1] Update flipbook animation
  (Sprite|SetFlipbook (Variables|Default|GetSprite) (select (Variables|Default|GetIsRunning) "/Game/Assets/Flipbooks/FB_PlayerRun.FB_PlayerRun" "/Game/Assets/Flipbooks/FB_PlayerIdle.FB_PlayerIdle"))
  (Collision|SetCollisionEnabled (Variables|Default|GetWallCollider) "NoCollision"))

(event EventUpdateJumpingAnimation
  ;[1 1 1] Update flipbook animation
  (Sprite|SetFlipbook (Variables|Default|GetSprite) (select (Variables|Default|GetIsJumping) "/Game/Assets/Flipbooks/FB_PlayerJump.FB_PlayerJump" "/Game/Assets/Flipbooks/FB_PlayerFall.FB_PlayerFall"))
  (Collision|SetCollisionEnabled (Variables|Default|GetWallCollider) "QueryOnly"))

(fn ConstructionScript
  (Variables|Default|SetHealth (Variables|Default|GetDefaultHealth)))

(fn Death
  (bind _camera (Variables|Default|GetCamera))
  (Transformation|DetachFromComponent _camera "KeepWorld" "KeepWorld" "KeepWorld" true)
  (Variables|Default|SetShouldRotate true)
  (Variables|Default|SetCameraLastLocation (Transformation|GetWorldLocation _camera))
  (Transformation|SetWorldLocation _camera (Variables|Default|GetCameraLastLocation) false false)
  (Utilities|FlowControl|DoOnce false
    (:Completed
      (Viewport|RemoveAllWidgets)
      (bind _returnvalue (UserInterface|CreateWidget "/Game/Assets/Widgets/WBP_RestartCounter.WBP_RestartCounter_C" (Game|GetPlayerController 0)))
      (bind _output_get (Variables|Default|SetCountdownWidget _returnvalue))
      (Default|UpdateCountdownText _output_get (Variables|Default|GetCountDown))
      (UserInterface|Viewport|AddtoPlayerScreen _output_get)
      (bind _returnvalue_2 (Utilities|Time|SetTimerbyFunctionName 0 "DeathProcess" 1.0 true))
      (Variables|Default|SetDeathCycleTimerHandle _returnvalue_2))))

(fn TakeSlowDamage
  (params (DamageCauser :type Actor%20Object%20Reference))
  (Game|Damage|ApplyDamage self (Variables|Default|GetBeamDamage) 0 DamageCauser))

(fn DeathProcess
  (bind _result (Math|Integer|DecrementInt (Variables|Default|GetCountDown))
    (:%20%20
      (bind _output_get (Variables|Default|SetCountDown _result))
      (Default|UpdateCountdownText (Variables|Default|GetCountdownWidget) _output_get)
      (if (<= (Variables|Default|GetCountDown) 0)
        (CallFunction|RespawnPlayer)
        (Utilities|Time|ClearandInvalidateTimerbyHandle (Variables|Default|GetDeathCycleTimerHandle))))))

(fn RespawnPlayer
  (Development|ExecuteConsoleCommand "RestartLevel" (Game|GetPlayerController 0)))

(fn HealHalfHealth
  (bind _output_get (Variables|Default|SetHealth (+ (Variables|Default|GetHealth) (/ (Variables|Default|GetDefaultHealth) 2.0))))
  (if (>= _output_get (Variables|Default|GetDefaultHealth))
    (bind _output_get_2 (Variables|Default|SetHealth (Variables|Default|GetDefaultHealth)))
    (Default|UpdateHealth (Variables|Default|GetHUDRef) _output_get_2)))

(fn PickupInterface
  (return false))