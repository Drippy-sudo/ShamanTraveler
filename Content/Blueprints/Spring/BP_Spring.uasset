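; BP_Spring is a launch pad that bounces the player when they enter its Box trigger.
; On overlap with a BP_PlayerBase, it zeroes the character's velocity, applies LaunchAmount as a velocity-change impulse and plays the Spring animation from the start.
; A DoOnce gate blocks repeat launches until the player leaves the Box or the animation finishes, which also rewinds and stops the animation.
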(event OnFinishedPlaying(Spring)
  (Components|Timeline|SetPlayRate (Variables|Default|GetSpring) 0.0)
  (Components|Timeline|SetPlaybackPosition (Variables|Default|GetSpring) 0.0 false)
  (CallFunction|ResetSpring))

(event OnComponentBeginOverlap(Box)
  (params (OverlappedComponent :type Primitive%20Component%20Object%20Reference) (OtherActor :type Actor%20Object%20Reference) (OtherComp :type Primitive%20Component%20Object%20Reference) (OtherBodyIndex :type Integer) (bFromSweep :type Boolean) (SweepResult :type Hit%20Result%20Structure%20%28by%20ref%29))
  (bind _spring (Variables|Default|GetSpring))
  (bind _asbp_player_base (Utilities|Casting|CastToBP_PlayerBase OtherActor))
  (Utilities|FlowControl|DoOnce false
    (:Completed
      (Variables|/Script/Engine.MovementComponent|SetVelocity (Variables|/Script/Engine.Character|GetCharacterMovement _asbp_player_base) "0, 0, 0")
      (Physics|AddImpulse (Variables|/Script/Engine.Character|GetCharacterMovement _asbp_player_base) (Variables|Default|GetLaunchAmount) true)
      (Components|Timeline|SetPlayRate _spring 1.0)
      (Components|Timeline|PlayfromStart _spring))))

(event OnComponentEndOverlap(Box)
  (params (OverlappedComponent :type Primitive%20Component%20Object%20Reference) (OtherActor :type Actor%20Object%20Reference) (OtherComp :type Primitive%20Component%20Object%20Reference) (OtherBodyIndex :type Integer))
  (Utilities|Casting|CastToBP_PlayerBase OtherActor)
  (CallFunction|ResetSpring))

(event Custom|ResetSpring
  (bind _spring (Variables|Default|GetSpring))
  (Utilities|FlowControl|DoOnce false) ; enters at Reset
)

(event EventBeginPlay
  (Components|Timeline|SetLooping (Variables|Default|GetSpring) false))

(event Collision|EventActorBeginOverlap
  (params (OtherActor :type Actor%20Object%20Reference)))

(event EventTick
  (params (DeltaSeconds :type Float%20%28single-precision%29)))

(fn ConstructionScript)